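; Tile_BP is a grid tile actor that sizes and positions itself from the Grid_BP that owns it.
; On BeginPlay it casts its owner to Grid_BP and uses TileSize as its X and Z scale, with Y scale zeroed.
; It then shifts half a tile along +X and -Z from its initial location and pins Y to a fixed depth, working in the XZ plane.
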(event `self.ReceiveBeginPlay`
  (bind _asgrid_bp (cast `/Game/Blueprints/Grid_BP` (`self.GetOwner`)))
  (bind (_x _y) (`KismetMathLibrary.BreakVector2D` (`Grid.TileSize` _asgrid_bp)))
  (`self.SetActorScale3D` (`KismetMathLibrary.MakeVector` _x 0.0 _y))
  (`self.K2_SetActorLocation` (`KismetMathLibrary.MakeVector` (+ (.x (`self.K2_GetActorLocation` self)) (/ _x 2.0)) 5.0 (- (.z (`self.K2_GetActorLocation` self)) (/ _y 2.0)))))

(fn `UserConstructionScript`)