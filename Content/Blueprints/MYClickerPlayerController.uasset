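; Player controller for a grid-based clicker game that creates the HUD, sets starting money and handles tile highlighting and object placement.
; Each tick it traces under the cursor, either highlighting the game mode grid's tile or snapping the HUD's placeable object to the tile center.
; Hovering always applies the invalid material, even over a hit.
; Left-click release asks the grid to place the stored object, ending placement mode on success.
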(event `self.ReceiveBeginPlay`
  (bind _returnvalue (`|CreateWidget` "/Game/Blueprints/HUD.HUD_C"))
  (bind _output_get (set `self.HUDReference` _returnvalue))
  (`UserWidget.AddToViewport` _output_get 0)
  (`WidgetBlueprintLibrary.SetInputMode_GameAndUIEx` (`GameplayStatics.GetPlayerController` 0) _output_get)
  (`self.SetMoney` 100)
  (bind _asmy_clicker_game_mode_base (cast `/Game/Blueprints/MyClickerGameModeBase` (`GameplayStatics.GetGameMode`)))
  (set `self.GridReference` (`/Game/Blueprints/MyClickerGameModeBase.GetGrid` _asmy_clicker_game_mode_base)))

(event `self.ReceiveTick`
  (params (DeltaSeconds :type "Float (single-precision)"))
  (if (`self.IsPlacingObject`)
    (`self.HoverObjectOnCursor` (`/Game/Blueprints/HUD.PlaceableObjectReference` (`self.HUDReference`)))
    (else
      (`self.HighlightGridUnderCursor`))))

(event `Key|LeftMouseButton`
  (params (Key :type "Key Structure"))
  (:`Released`
    (if (`self.IsPlacingObject`)
      (if (`self.IsSelectionValid`)
        (bind _returnvalue (`GridV2.TryPlaceObjectAtWorldLocation` (`self.GridReference`) (`self.PlaceableObject`) (`self.SelectedTile`)))
        (if _returnvalue
          (set `self.IsPlacingObject` false))))))

(fn `HighlightGridUnderCursor`
  (locals (Grid :type "/Game/Blueprints/GridV2_BP Object Reference") (HitLocation :type "Vector Structure" :default (0.0 0.0 0.0)))
  (bind _gridreference (`self.GridReference`))
  (cast `/Game/Blueprints/MyClickerGameModeBase` (`GameplayStatics.GetGameMode`))
  (bind _asmyclicker_player_controller (cast `/Game/Blueprints/MYClickerPlayerController` (`GameplayStatics.GetPlayerController` 0)))
  (bind (_hitresult _returnvalue) (`self.GetHitResultUnderCursorByChannel` _asmyclicker_player_controller "TraceTypeQuery2" true))
  (if _returnvalue
    (bind _output_get (set `local.HitLocation` (`.Location` (`GameplayStatics.BreakHitResult` _hitresult))))
    (bind (_outrow _outcolumn) (`GridV2.WorldLocationToTile` _gridreference _output_get))
    (`GridV2.SetSelectedTile` _gridreference _outrow _outcolumn)
    (else
      (`GridV2.SetSelectedTile` (`self.GridReference`) -1 -1))))

(fn `HoverObjectOnCursor`
  (params (PlaceableObject :type "PlaceableObject Object Reference"))
  (locals (PlaceableObjectReference :type "PlaceableObject Object Reference") (Grid :type "/Game/Blueprints/GridV2_BP Object Reference") (HitLocation :type "Vector Structure" :default (0.0 0.0 0.0)))
  (bind _placeableobjectreference (`local.PlaceableObjectReference`))
  (bind _gridreference (`self.GridReference`))
  (set `local.PlaceableObjectReference` PlaceableObject)
  (cast `/Game/Blueprints/MyClickerGameModeBase` (`GameplayStatics.GetGameMode`))
  (bind _asmyclicker_player_controller (cast `/Game/Blueprints/MYClickerPlayerController` (`GameplayStatics.GetPlayerController` 0)))
  (bind (_hitresult _returnvalue) (`self.GetHitResultUnderCursorByChannel` _asmyclicker_player_controller "TraceTypeQuery2" true))
  (set `self.IsSelectionValid` _returnvalue)
  (if _returnvalue
    (bind _output_get (set `local.HitLocation` (`.Location` (`GameplayStatics.BreakHitResult` _hitresult))))
    (bind (_outrow _outcolumn) (`GridV2.WorldLocationToTile` _gridreference _output_get))
    (bind _outgridlocation (`GridV2.TileToGridLocation` _gridreference _outrow _outcolumn true))
    (`SceneComponent.K2_SetWorldLocationAndRotation` :`self` (`Actor.RootComponent` _placeableobjectreference) :`NewLocation` (`KismetMathLibrary.MakeVector` (`KismetMathLibrary.BreakVector2D` _outgridlocation) (`.Y` (`KismetMathLibrary.BreakVector2D` _outgridlocation))))
    (`PrimitiveComponent.SetMaterial` (`PlaceableObject.StaticMeshComponent` _placeableobjectreference) 0 "/Game/Materials/Invalid_Material_Instance.Invalid_Material_Instance")
    (set `self.SelectedTile` (`KismetMathLibrary.MakeVector` (`KismetMathLibrary.BreakVector2D` _outgridlocation) (`.Y` (`KismetMathLibrary.BreakVector2D` _outgridlocation)) 50.0))
    (else
      (`GridV2.SetSelectedTile` (`self.GridReference`) -1 -1))))

(fn `Set Placeable Object`
  (params (PlaceableObject :type "PlaceableObject Object Reference"))
  (set `self.PlaceableObject` PlaceableObject)
  (return))

(fn `UserConstructionScript`)